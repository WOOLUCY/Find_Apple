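; Temporary slime AI character that takes damage, shows its health through its material and dies at zero health.
; Tick swaps the mesh material across five slime variants by exact-matching Health in steps of 20.
; AnyDamage subtracts health behind a DoOnce that resets after a short delay, setting IsAttacked during that window.
; Lethal damage disables capsule collision, plays the damaged animation, then destroys the actor after a delay.
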(event EventBeginPlay)

(event Collision|EventActorBeginOverlap
  (params (OtherActor :type Actor%20Object%20Reference)))

(event EventTick
  (params (DeltaSeconds :type Float%20%28single-precision%29))
  (Utilities|FlowControl|Sequence
    (:then_0
      (if (== (Variables|Default|GetHealth) 100)
        (Rendering|Material|SetMaterial (Variables|Character|GetMesh) 0 "/Game/Woo/Monster/Slime/MI_Slime01.MI_Slime01")))
    (:then_1
      (if (== (Variables|Default|GetHealth) 80)
        (Rendering|Material|SetMaterial (Variables|Character|GetMesh) 0 "/Game/Woo/Monster/Slime/MI_Slime02.MI_Slime02")))
    (:then_2
      (if (== (Variables|Default|GetHealth) 60)
        (Rendering|Material|SetMaterial (Variables|Character|GetMesh) 0 "/Game/Woo/Monster/Slime/MI_Slime03.MI_Slime03")))
    (:then_3
      (if (== (Variables|Default|GetHealth) 40)
        (Rendering|Material|SetMaterial (Variables|Character|GetMesh) 0 "/Game/Woo/Monster/Slime/MI_Slime04.MI_Slime04")))
    (:then_4
      (if (== (Variables|Default|GetHealth) 20)
        (Rendering|Material|SetMaterial (Variables|Character|GetMesh) 0 "/Game/Woo/Monster/Slime/MI_Slime05.MI_Slime05")))))

(event Game|Damage|EventAnyDamage
  (params (Damage :type Float%20%28single-precision%29) (DamageType :type Damage%20Type%20Object%20Reference) (InstigatedBy :type Controller%20Object%20Reference) (DamageCauser :type Actor%20Object%20Reference))
  (Utilities|FlowControl|DoOnce false :!label _label
    (:Completed
      (Variables|Default|SetIs%20Attacked? true)
      (Development|PrintString (Utilities|String|ToString(Integer) (- (Variables|Default|GetHealth) (Variables|Default|GetDamage))))
      (if (<= (- (Variables|Default|GetHealth) (Variables|Default|GetDamage)) 0)
        (bind _output_get (Variables|Default|SetHealth (- (Variables|Default|GetHealth) (Variables|Default|GetDamage))))
        (Variables|Default|SetHealth _output_get)
        (Audio|Components|Audio|Stop (Variables|Character|GetMesh))
        (Collision|SetCollisionEnabled (Variables|Collision|GetCapsuleComponent) "NoCollision")
        (Components|Animation|PlayAnimation (Variables|Character|GetMesh) "/Game/Monsters/Slime/Damged.Damged" false)
        (Utilities|FlowControl|Delay 1.0)
        (Actor|DestroyActor)
        (else
          (Variables|Default|SetHealth (- (Variables|Default|GetHealth) (Variables|Default|GetDamage)))
          (Utilities|FlowControl|Delay 0.5)
          (Variables|Default|SetIs%20Attacked? false)
          (goto _label Reset))))))

(fn ConstructionScript)