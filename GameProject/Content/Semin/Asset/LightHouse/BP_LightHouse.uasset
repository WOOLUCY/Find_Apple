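; BP_LightHouse is a lighthouse actor that plays a short camera cutscene when the player character enters its Box trigger.
; The overlap stops and disables character movement, switches input to Game and UI, and blends the view to the lighthouse camera.
; A timeline eases Camera toward Camera1's transform by lerping from its current transform each update.
; On finish, it blends back to the player and restores walking and game-only input.
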(event OnComponentBeginOverlap(Box)
  (params (OverlappedComponent :type Primitive%20Component%20Object%20Reference) (OtherActor :type Actor%20Object%20Reference) (OtherComp :type Primitive%20Component%20Object%20Reference) (OtherBodyIndex :type Integer) (bFromSweep :type Boolean) (SweepResult :type Hit%20Result%20Structure%20%28by%20ref%29))
  (bind _returnvalue (Game|GetPlayerController 0))
  (bind _returnvalue_2 (Game|GetPlayerCharacter 0))
  (bind _asfind_apple_player_controller (Utilities|Casting|CastToFindApplePlayerController _returnvalue))
  (bind _asfind_apple_character (Utilities|Casting|CastToFindAppleCharacter _returnvalue_2))
  (bind _charactermovement (Variables|/Script/Engine.Character|GetCharacterMovement _asfind_apple_character))
  (bind _asfind_apple_character_2 (Utilities|Casting|CastToFindAppleCharacter OtherActor))
  (Pawn|Components|CharacterMovement|DisableMovement (Variables|/Script/Engine.Character|GetCharacterMovement _asfind_apple_character_2))
  (Variables|/Script/Engine.MovementComponent|SetVelocity (Variables|/Script/Engine.Character|GetCharacterMovement _asfind_apple_character_2) "0, 0, 0")
  (Input|SetInputModeGameandUI (Game|GetPlayerController 0) 0 "DoNotLock" true false)
  (Game|Player|SetViewTargetwithBlend (.AsFind%20Apple%20Player%20Controller (Utilities|Casting|CastToFindApplePlayerController (Game|GetPlayerController 0))) (Components|GetOwner (Variables|Default|GetCamera)) 3.0 "VTBlend_Linear" 0.0 false)
  (Utilities|FlowControl|Delay 3.0)
  (bind _새_트랙_1 (Timeline|TimeLine PlayFromStart)
    (:Update
      (Transformation|SetWorldLocationAndRotation (Variables|Default|GetCamera) (Math|Vector|Lerp(Vector) (Transformation|GetWorldLocation (Variables|Default|GetCamera)) (Transformation|GetWorldLocation (Variables|Default|GetCamera1)) _새_트랙_1) (Math|Rotator|Lerp(Rotator) (Transformation|GetWorldRotation (Variables|Default|GetCamera)) (Transformation|GetWorldRotation (Variables|Default|GetCamera1)) _새_트랙_1 true) false false))
    (:Finished
      (Utilities|FlowControl|Delay 1.0)
      (Game|Player|SetViewTargetwithBlend _asfind_apple_player_controller (Components|GetOwner (Variables|/Script/GameProject.FindAppleCharacter|GetCameraComponent _asfind_apple_character)) 3.0 "VTBlend_Linear" 0.0 false)
      (Pawn|Components|CharacterMovement|SetMovementMode _charactermovement "MOVE_Walking" 0)
      (Input|SetInputModeGameOnly _asfind_apple_player_controller false)
      (Variables|/Script/Engine.MovementComponent|SetVelocity _charactermovement "0, 0, 0"))))

(event Custom|SetCamera)

(event EventBeginPlay)

(event Collision|EventActorBeginOverlap
  (params (OtherActor :type Actor%20Object%20Reference)))

(event EventTick
  (params (DeltaSeconds :type Float%20%28single-precision%29)))

(fn ConstructionScript)