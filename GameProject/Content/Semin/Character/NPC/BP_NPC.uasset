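; NPC actor that shows line-by-line dialogue from a data table in a WBP_Dialogue widget.
; BeginPlay caches the table rows matching its NPCID, and each InteractionDialogue call advances the line counter and creates or updates the widget.
; DialogueGetLine matches conversation and line IDs, closing the widget and resetting the counter unless exactly one line matches.
; Ending overlap with the dialogue box removes the widget; begin overlap only casts.
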(event OnComponentBeginOverlap(OverlapDialogueBox)
  (params (OverlappedComponent :type Primitive%20Component%20Object%20Reference) (OtherActor :type Actor%20Object%20Reference) (OtherComp :type Primitive%20Component%20Object%20Reference) (OtherBodyIndex :type Integer) (bFromSweep :type Boolean) (SweepResult :type Hit%20Result%20Structure%20%28by%20ref%29))
  (Utilities|Casting|CastToBP_FindAppleCharacter_Quest OtherActor))

(event OnComponentEndOverlap(OverlapDialogueBox)
  (params (OverlappedComponent :type Primitive%20Component%20Object%20Reference) (OtherActor :type Actor%20Object%20Reference) (OtherComp :type Primitive%20Component%20Object%20Reference) (OtherBodyIndex :type Integer))
  (Utilities|IsValid (Variables|Default|GetDialogueWidget)
    (:Is%20Valid
      (Widget|RemovefromParent (Variables|Default|GetDialogueWidget))
      (Variables|Default|SetDialogueWidget 0))))

(event EventBeginPlay
  (bind _outrownames (DataTable|GetDataTableRowNames "/Game/Semin/UI/Dialogue_File.Dialogue_File"))
  (for _array_element _outrownames
    (bind _returnvalue (Utilities|GetDataTableRow "/Game/Semin/UI/Dialogue_File.Dialogue_File" _array_element)
      (:then
        (if (== (.NPC_ID (Utilities|Struct|BreakDialogueStruct _returnvalue)) (Variables|Default|GetNPC_ID))
          (Utilities|Array|Add (Variables|Default|GetMyDialogue) _array_element))))))

(event Collision|EventActorBeginOverlap
  (params (OtherActor :type Actor%20Object%20Reference)))

(event EventTick
  (params (DeltaSeconds :type Float%20%28single-precision%29)))

(event EventInteractionDialogue
  (Math|Integer|IncrementInt (Variables|Default|GetLineCurrent)
    (:%20%20
      (CallFunction|DialogueCreate))))

(fn ConstructionScript)

(fn DialogueCreate
  (Utilities|IsValid (Variables|Default|GetDialogueWidget)
    (:Is%20Valid
      (bind _returnedline (CallFunction|DialogueGetLine))
      (if (not (Utilities|Text|TextIsEmpty _returnedline))
        (Variables|/Game/Semin/UI/WBP_Dialogue.WBP_Dialogue_C|SetDialogueText (Variables|Default|GetDialogueWidget) _returnedline)))
    (:Is%20Not%20Valid
      (bind _returnvalue (UserInterface|CreateWidget "/Game/Semin/UI/WBP_Dialogue.WBP_Dialogue_C" (Game|GetPlayerController 0)))
      (bind _output_get (Variables|Default|SetDialogueWidget _returnvalue))
      (UserInterface|Viewport|AddtoViewport _output_get 0)
      (bind _returnedline_2 (CallFunction|DialogueGetLine))
      (if (not (Utilities|Text|TextIsEmpty _returnedline_2))
        (Variables|/Game/Semin/UI/WBP_Dialogue.WBP_Dialogue_C|SetDialogueText (Variables|Default|GetDialogueWidget) _returnedline_2)
        (Variables|/Game/Semin/UI/WBP_Dialogue.WBP_Dialogue_C|SetNPCText (Variables|Default|GetDialogueWidget) (Variables|Default|GetMyNameText))))))

(fn DialogueGetLine
  (for _array_element (Variables|Default|GetMyDialogue)
    (bind _returnvalue (Utilities|GetDataTableRow "/Game/Semin/UI/Dialogue_File.Dialogue_File" _array_element)
      (:then
        (if (and (== (.Conversation_ID (Utilities|Struct|BreakDialogueStruct _returnvalue)) (Variables|Default|GetConversation_ID)) (== (.Line_ID (Utilities|Struct|BreakDialogueStruct _returnvalue)) (Variables|Default|GetLineCurrent)))
          (Utilities|Array|Add (LocalVariables|GetReturnedLines) (.Dialogue (Utilities|Struct|BreakDialogueStruct _returnvalue)))
          (Development|PrintString (Utilities|String|ToString(Text) (.Dialogue (Utilities|Struct|BreakDialogueStruct _returnvalue))))))))
  (Variables|Default|SetMyNameText (.NPC_Name (Utilities|Struct|BreakDialogueStruct _returnvalue)))
  (if (== (Utilities|Array|Length (LocalVariables|GetReturnedLines)) 1)
    (return (Utilities|Array|Get(acopy) (LocalVariables|GetReturnedLines)))
    (else
      (Widget|RemovefromParent (Variables|Default|GetDialogueWidget))
      (Variables|Default|SetDialogueWidget 0)
      (Variables|Default|SetLineCurrent 0))))