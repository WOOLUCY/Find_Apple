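; BP_FindAppleCharacter_Quest is a character Blueprint for a quest, used as a test bed for inventory interaction.
; Quest interaction input messages a valid looked-at actor when PressE is set, plays a sound and caches InventoryComponent keys.
; A second handler on that input triggers dialogue on overlapping Interaction_i actors, found by scanning all implementers.
; Inventory input adds a new WBP_Inventory to the viewport each time; the removal logic is disconnected.
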(event Input|EnhancedActionEvents|EnhancedInputActionIA_QuestInteraction
  (params (ActionValue :type Boolean) (ElapsedSeconds :type Float%20%28double-precision%29) (TriggeredSeconds :type Float%20%28double-precision%29) (InputAction :type Input%20Action%20Object%20Reference :default "/Game/Semin/KeyInput/IA_QuestInteraction.IA_QuestInteraction"))
  ;[1 1 1] 세민 - 인벤토리 블프로 먼저 테스트 중
  (:Started
    (if (Variables|Default|GetPressE)
      (bind _lookatactorpresse (Variables|Default|GetLookatActorPressE)
        (:then
          (Class|InteractionI|Interactionwith(Message) _lookatactorpresse self)
          (bind _keys (Utilities|Map|Keys (Variables|/Game/Semin/UI/Inventory/InventoryComponent.InventoryComponent_C|GetInventoryContent (Variables|Default|GetInventoryComponent))))
          (Audio|PlaySoundatLocation "/Engine/VREditor/Sounds/UI/Dockable_Window_Open.Dockable_Window_Open" (Transformation|GetActorLocation (Game|GetPlayerCharacter 0)) "0, 0, 0" 1.0 1.0 0.0 0 0 0 0)
          (Development|PrintString "Hello"))
        (:else)))))

(event Input|EnhancedActionEvents|EnhancedInputActionIA_QuestInteraction
  (params (ActionValue :type Boolean) (ElapsedSeconds :type Float%20%28double-precision%29) (TriggeredSeconds :type Float%20%28double-precision%29) (InputAction :type Input%20Action%20Object%20Reference :default "/Game/Semin/KeyInput/IA_QuestInteraction.IA_QuestInteraction"))
  (:Started
    (bind _outactors (Actor|GetAllActorswithInterface "/Game/Semin/UI/Interaction_i.Interaction_i_C"))
    (for _array_element _outactors
      (if (Collision|IsOverlappingActor _array_element self :!class /Script/Engine.Actor)
        (Class|InteractionI|InteractionDialogue(Message) _array_element)))))

(event Input|EnhancedActionEvents|EnhancedInputActionIA_Inventory
  (params (ActionValue :type Boolean) (ElapsedSeconds :type Float%20%28double-precision%29) (TriggeredSeconds :type Float%20%28double-precision%29) (InputAction :type Input%20Action%20Object%20Reference :default "/Game/Semin/KeyInput/IA_Inventory.IA_Inventory"))
  (:Started
    (bind _returnvalue (UserInterface|CreateWidget "/Game/Semin/UI/Inventory/UI/WBP_Inventory.WBP_Inventory_C"))
    (bind _output_get (Variables|Default|SetPlayerInventory _returnvalue))
    (UserInterface|Viewport|AddtoViewport _returnvalue 0)))

(event EventBeginPlay)

(event Collision|EventActorBeginOverlap
  (params (OtherActor :type Actor%20Object%20Reference)))

(event EventTick
  (params (DeltaSeconds :type Float%20%28single-precision%29)))

(fn ConstructionScript)